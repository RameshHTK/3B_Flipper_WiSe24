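; BP_Pillar is a pillar actor that carries two point lights with configurable appearance.
; On BeginPlay it applies its LightIntensity, LightColor and LightsCastShadows variables to both PointLight and PointLight1.
; The settings are applied only at runtime, since the construction script is empty and Tick does nothing.
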(event EventBeginPlay
  (Rendering|Components|Light|SetIntensity (Variables|Default|GetPointLight) (Variables|Default|GetLight%20Intensity))
  (Rendering|Components|Light|SetLightColor (Variables|Default|GetPointLight) (Variables|Default|GetLight%20Color) true)
  (Rendering|Components|Light|SetCastShadows (Variables|Default|GetPointLight) (Variables|Default|GetLights%20Cast%20Shadows)))

(event EventTick
  (params (DeltaSeconds :type Float%20%28single-precision%29)))

(fn ConstructionScript)