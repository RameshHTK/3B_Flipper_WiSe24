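; BP_Ball is a ball Blueprint that launches its Sphere upward with a charged spacebar press.
; Tick accumulates how long the spacebar is held.
; On release, that duration is normalized against a maximum charge time, clamped and scaled by a maximum strength into a vertical impulse on the Sphere, then the charge resets.
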(event EventTick
  (params (DeltaSeconds :type Float%20%28single-precision%29))
  (if (Variables|Default|GetIsSpacebarPressed)
    (Variables|Default|SetSpacebarHeldDuration (+ DeltaSeconds (Variables|Default|GetSpacebarHeldDuration)))))

(event Input|KeyboardEvents|SpaceBar
  (params (Key :type Key%20Structure :default "None"))
  (:Pressed
    (Variables|Default|SetIsSpacebarPressed true))
  (:Released
    (Physics|AddImpulse (Variables|Default|GetSphere) (Math|Vector|MakeVector 0.0 0.0 (* (Variables|Default|GetMaxImpulseStrength) (Math|Float|Clamp(Float) (/ (Variables|Default|GetSpacebarHeldDuration) (Variables|Default|GetMaxChargeDuration)) 0.0 1.0))) "None" false)
    (Variables|Default|SetIsSpacebarPressed false)
    (Variables|Default|SetSpacebarHeldDuration 0.0)))

(fn ConstructionScript)